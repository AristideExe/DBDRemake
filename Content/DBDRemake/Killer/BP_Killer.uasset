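; Killer character for a Dead by Daylight remake, with a lunge attack and actions to destroy pallets and break generators.
; Holding attack calls SR_StartAttacking, which blocks move input and launches the character forward on a looping timer.
; Release or max duration ends the lunge with a camera sphere trace, damaging a hit survivor on authority.
; Pallet and generator actions multicast from authority, turning the killer and pausing movement briefly.
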(event `EnhancedInput|/Game/DBDRemake/Input/Actions/IA_Attack`
  (params (ActionValue :type Boolean) (ElapsedSeconds :type "Float (double-precision)") (TriggeredSeconds :type "Float (double-precision)") (InputAction :type "InputAction Object Reference" :default "/Game/DBDRemake/Input/Actions/IA_Attack.IA_Attack"))
  (:`Started`
    (if (not (`self.IsAttacking?`))
      (`self.SR_StartAttacking`)))
  (:`Canceled`
    (`self.MC_StopAttacking` :!label _label))
  (:`Completed`
    (goto _label)))

(event `DestroyPallet`
  (params (Pallet :type "/Game/DBDRemake/Interactive/Pallet/BP_Pallet Object Reference") (BeginLocation :type "Vector Structure"))
  ;[0.15 0.15 0.15 0.5 50] Destroy Pallet
  (`/Engine/EditorBlueprintResources/ActorMacros.Switch Has Authority`
    (:`Authority`
      (`self.MC_DestroyPallet` Pallet BeginLocation))))

(event `MC_DestroyPallet`
  (params (Pallet :type "/Game/DBDRemake/Interactive/Pallet/BP_Pallet Object Reference") (BeginLocation :type "Vector Structure"))
  ;[0.15 0.15 0.15 0.5 50] Destroy Pallet
  (`self.K2_SetActorLocation` BeginLocation)
  (`self.K2_SetActorRotation` (`KismetMathLibrary.FindLookAtRotation` BeginLocation (`self.K2_GetActorLocation` Pallet)))
  (`CharacterMovementComponent.DisableMovement` (`self.CharacterMovement`))
  (`KismetSystemLibrary.Delay` 1.0)
  (`/Engine/EditorBlueprintResources/StandardMacros.IsValid` Pallet
    (:`Is Valid`
      (`self.K2_DestroyActor` Pallet)
      (`CharacterMovementComponent.SetMovementMode` (`self.CharacterMovement`) "MOVE_Walking" 0))))

(event `SR_StartAttacking`
  (set `self.IsAttacking?` true)
  (bind _returnvalue (`KismetSystemLibrary.K2_SetTimerDelegate` (delegate `Attack`) 0.1 true))
  (set `self.AttackingTimerHandle` _returnvalue)
  (`KismetSystemLibrary.Delay` (`self.AttackMaxDuration`))
  (`self.MC_StopAttacking`))

(event `Attack`
  (`self.LaunchCharacter` (* (`self.GetActorForwardVector`) (`self.AttackForce`)) true true))

(event `DestroyGenerator`
  (params (Pallet :type "/Game/DBDRemake/Interactive/Generator/BP_Generator Object Reference") (BreakLocation :type "Vector Structure"))
  ;[0.15 0.15 0.15 0.5 50] Destroy Generator
  (`/Engine/EditorBlueprintResources/ActorMacros.Switch Has Authority`
    (:`Authority`
      (`self.MC_DestroyGenerator` Pallet BreakLocation))))

(event `MC_StopAttacking`
  (bind _followcamera (`self.FollowCamera`))
  (bind _returnvalue (`SceneComponent.K2_GetComponentLocation` _followcamera))
  (if (`self.IsAttacking?`)
    (set `self.IsAttacking?` false)
    (`KismetSystemLibrary.K2_ClearAndInvalidateTimerHandle` (`self.AttackingTimerHandle`))
    (bind (_outhit _returnvalue_2) (`KismetSystemLibrary.SphereTraceSingle` :`Start` _returnvalue :`End` (+ _returnvalue (* (`SceneComponent.GetForwardVector` _followcamera) (`self.AttackDistance`))) :`Radius` 20.0 :`TraceChannel` "TraceTypeQuery2" :`DrawDebugType` "ForDuration"))
    (if _returnvalue_2
      (`/Engine/EditorBlueprintResources/ActorMacros.Switch Has Authority`
        (:`Authority`
          (bind _asbp_survivor (cast `/Game/DBDRemake/Survivor/BP_Survivor` (`.HitActor` (`GameplayStatics.BreakHitResult` _outhit))))
          (`/Game/DBDRemake/Survivor/BP_Survivor.TakeDamage` _asbp_survivor))))))

(event `MC_DestroyGenerator`
  (params (Pallet :type "/Game/DBDRemake/Interactive/Generator/BP_Generator Object Reference") (BreakLocation :type "Vector Structure"))
  ;[0.15 0.15 0.15 0.5 50] Destroy Generator
  (`self.K2_SetActorRotation` (`KismetMathLibrary.FindLookAtRotation` BreakLocation (`self.K2_GetActorLocation` Pallet)))
  (`CharacterMovementComponent.DisableMovement` (`self.CharacterMovement`))
  (`KismetSystemLibrary.Delay` 1.0)
  (`/Engine/EditorBlueprintResources/StandardMacros.IsValid` Pallet
    (:`Is Valid`
      (`/Game/DBDRemake/Interactive/Generator/BP_Generator.BreakGenerator` Pallet)
      (`CharacterMovementComponent.SetMovementMode` (`self.CharacterMovement`) "MOVE_Walking" 0))))

(fn `Move`
  (params (`X Axis` :type "Float (double-precision)") (`Y Axis` :type "Float (double-precision)"))
  (if (not (`self.IsAttacking?`))
    (`parent.Move` `X Axis` `Y Axis`)))

(fn `UserConstructionScript`)