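; Lobby game mode that gathers joining players and launches the match.
; PostLogin adds each controller to a Players array and OnLogout removes it.
; Once at least two players are present, it prints a launch message, waits briefly, then runs a servertravel console command to LVL_GAME.
; The pending launch has no cancel or recheck if a player leaves during the delay.
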(event `self.K2_PostLogin`
  (params (NewPlayer :type "PlayerController Object Reference"))
  (bind _players (`self.Players`))
  (`KismetArrayLibrary.Array_Add` _players NewPlayer)
  (if (>= (`KismetArrayLibrary.Array_Length` _players) 2)
    (`KismetSystemLibrary.PrintString` "Launch Game")
    (`KismetSystemLibrary.Delay` 1.0)
    (`self.Travel`)))

(event `Travel`
  (`KismetSystemLibrary.ExecuteConsoleCommand` "servertravel LVL_GAME" null))

(event `self.K2_OnLogout`
  (params (ExitingController :type "Controller Object Reference"))
  (bind _asplayer_controller (cast `PlayerController` ExitingController))
  (`KismetArrayLibrary.Array_RemoveItem` (`self.Players`) _asplayer_controller))

(fn `UserConstructionScript`)