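; BP_Window is an interactable window that survivors can vault through in a Dead by Daylight remake.
; Its Box overlap registers and unregisters it with the player's BPCInteract component, which it supplies with an input action, key label and prompt text.
; On interaction, only a BP_Survivor triggers GoThroughWindow, with GetDirection using the nearer of points A and B as start and the other as end.
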(event `self.Box.OnComponentBeginOverlap`
  (params (OverlappedComponent :type "PrimitiveComponent Object Reference") (OtherActor :type "Actor Object Reference") (OtherComp :type "PrimitiveComponent Object Reference") (OtherBodyIndex :type Integer) (bFromSweep :type Boolean) (SweepResult :type "HitResult Structure (by ref)"))
  (bind _asbp_player (cast `/Game/DBDRemake/Common/BP_Player` OtherActor))
  (`/Game/DBDRemake/Common/BPC_Interact.InteractObjectBeginOverlap` (`/Game/DBDRemake/Common/BP_Player.BPC_Interact` _asbp_player) self _asbp_player))

(event `self.Box.OnComponentEndOverlap`
  (params (OverlappedComponent :type "PrimitiveComponent Object Reference") (OtherActor :type "Actor Object Reference") (OtherComp :type "PrimitiveComponent Object Reference") (OtherBodyIndex :type Integer))
  (bind _asbp_player (cast `/Game/DBDRemake/Common/BP_Player` OtherActor))
  (`/Game/DBDRemake/Common/BPC_Interact.InteractObjectEndOverlap` (`/Game/DBDRemake/Common/BP_Player.BPC_Interact` _asbp_player)))

(event `/Game/DBDRemake/Common/BPI_Interact.BeginInteraction`
  (params (Player :type "/Game/DBDRemake/Common/BP_Player Object Reference") (`ServerInteract?` :type Boolean))
  (bind _asbp_survivor (cast `/Game/DBDRemake/Survivor/BP_Survivor` Player))
  (bind (_begin _end) (`self.GetDirection` _asbp_survivor))
  (`/Game/DBDRemake/Survivor/BP_Survivor.GoThroughWindow` _asbp_survivor _begin _end))

(event `/Game/DBDRemake/Common/BPI_Interact.EndInteraction`
  (params (Player :type "/Game/DBDRemake/Common/BP_Player Object Reference") (`ServerInteract?` :type Boolean)))

(fn `GetDirection`
  (params (Player :type "Actor Object Reference"))
  (returns (Begin :type "Vector Structure") (End :type "Vector Structure"))
  (bind _returnvalue (`self.K2_GetActorLocation` Player))
  (bind _returnvalue_2 (`SceneComponent.K2_GetComponentLocation` (`self.A`)))
  (bind _returnvalue_3 (`SceneComponent.K2_GetComponentLocation` (`self.B`)))
  (if (< (`KismetMathLibrary.Vector_Distance` _returnvalue (`SceneComponent.K2_GetComponentLocation` (`self.A`))) (`KismetMathLibrary.Vector_Distance` _returnvalue (`SceneComponent.K2_GetComponentLocation` (`self.B`))))
    (return _returnvalue_2 _returnvalue_3)
    (else
      (return _returnvalue_3 _returnvalue_2))))

(fn `GetInputAction`
  (params (Role :type "/Game/DBDRemake/Common/ENUM_Role Enum" :default "NewEnumerator0"))
  (returns (Input :type "InputAction Object Reference"))
  (return "/Game/DBDRemake/Input/Actions/IA_Interact1.IA_Interact1"))

(fn `GetInteractionInput`
  (params (Role :type "/Game/DBDRemake/Common/ENUM_Role Enum" :default "NewEnumerator0"))
  (returns (Input :type String))
  (return "SPACE"))

(fn `GetInteractionText`
  (params (Role :type "/Game/DBDRemake/Common/ENUM_Role Enum" :default "NewEnumerator0"))
  (returns (Text :type String))
  (return "TRAVERSER"))

(fn `UserConstructionScript`)