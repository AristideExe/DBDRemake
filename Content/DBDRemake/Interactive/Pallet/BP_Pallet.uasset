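; Interactive pallet for a Dead by Daylight remake: survivors drop it, then vault it, and killers can destroy it once dropped.
; A box overlap registers it with each player's interact component, for killers only after the drop.
; Server-side interaction branches on role, using the nearer of points A/B to orient vaults and destruction.
; The drop event, apparently multicast, enables blocking collision and tips the mesh with a timeline; prompts are French.
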(event `self.Box.OnComponentBeginOverlap`
  (params (OverlappedComponent :type "PrimitiveComponent Object Reference") (OtherActor :type "Actor Object Reference") (OtherComp :type "PrimitiveComponent Object Reference") (OtherBodyIndex :type Integer) (bFromSweep :type Boolean) (SweepResult :type "HitResult Structure (by ref)"))
  (bind _asbp_player (cast `/Game/DBDRemake/Common/BP_Player` OtherActor))
  (switch `/Game/DBDRemake/Common/ENUM_Role` (`/Game/DBDRemake/Common/BP_Player.PlayerRole` _asbp_player)
    (:`NewEnumerator0`
      (bind _bpc_interact (`/Game/DBDRemake/Common/BP_Player.BPC_Interact` _asbp_player))
      (`/Game/DBDRemake/Common/BPC_Interact.InteractObjectBeginOverlap` _bpc_interact self _asbp_player))
    (:`NewEnumerator1`
      (if (`self.IsDropped`)
        (`/Game/DBDRemake/Common/BPC_Interact.InteractObjectBeginOverlap` _bpc_interact self _asbp_player)))))

(event `self.Box.OnComponentEndOverlap`
  (params (OverlappedComponent :type "PrimitiveComponent Object Reference") (OtherActor :type "Actor Object Reference") (OtherComp :type "PrimitiveComponent Object Reference") (OtherBodyIndex :type Integer))
  (bind _asbp_player (cast `/Game/DBDRemake/Common/BP_Player` OtherActor))
  (`/Game/DBDRemake/Common/BPC_Interact.InteractObjectEndOverlap` (`/Game/DBDRemake/Common/BP_Player.BPC_Interact` _asbp_player)))

(event `/Game/DBDRemake/Common/BPI_Interact.BeginInteraction`
  (params (Player :type "/Game/DBDRemake/Common/BP_Player Object Reference") (`ServerInteract?` :type Boolean))
  (if `ServerInteract?`
    (switch `/Game/DBDRemake/Common/ENUM_Role` (`/Game/DBDRemake/Common/BP_Player.PlayerRole` Player)
      (:`NewEnumerator0`
        (bind _asbp_survivor (cast `/Game/DBDRemake/Survivor/BP_Survivor` Player))
        (if (`self.IsDropped`)
          (bind (_begin _end) (`self.GetDirection` _asbp_survivor))
          (`/Game/DBDRemake/Survivor/BP_Survivor.VaultPallet` _asbp_survivor _begin _end)
          (else
            (`self.MC_DropPallet`))))
      (:`NewEnumerator1`
        (bind _asbp_killer (cast `/Game/DBDRemake/Killer/BP_Killer` Player))
        (`/Game/DBDRemake/Killer/BP_Killer.DestroyPallet` _asbp_killer self (`self.GetClosestPoint` _asbp_killer))))))

(event `MC_DropPallet`
  (bind _sm_pallet (`self.SM_Pallet`))
  (bind _droppedcollision (`self.DroppedCollision`))
  (set `self.IsDropped` true)
  (`PrimitiveComponent.SetCollisionEnabled` _droppedcollision "QueryAndPhysics")
  (`PrimitiveComponent.SetCollisionObjectType` _droppedcollision "ECC_Pawn")
  (bind (_direction _alpha) (`Timeline|Drop Pallet`)
    (:`Update`
      (`SceneComponent.K2_SetRelativeRotation` _sm_pallet (`KismetMathLibrary.RLerp` (struct) (struct :`Pitch` -70.0) _alpha) false false)
      (`SceneComponent.K2_SetRelativeLocation` _sm_pallet (`KismetMathLibrary.VLerp` (0.0 0.0 0.0) (-15.0 0.0 0.0) _alpha) false false))))

(event `/Game/DBDRemake/Common/BPI_Interact.EndInteraction`
  (params (Player :type "/Game/DBDRemake/Common/BP_Player Object Reference") (`ServerInteract?` :type Boolean)))

(fn `GetClosestPoint`
  (params (Player :type "Actor Object Reference"))
  (returns (ClosetPoint :type "Vector Structure"))
  (bind _returnvalue (`self.K2_GetActorLocation` Player))
  (if (< (`KismetMathLibrary.Vector_Distance` _returnvalue (`SceneComponent.K2_GetComponentLocation` (`self.A`))) (`KismetMathLibrary.Vector_Distance` _returnvalue (`SceneComponent.K2_GetComponentLocation` (`self.B`))))
    (return (`SceneComponent.K2_GetComponentLocation` (`self.A`)))
    (else
      (return (`SceneComponent.K2_GetComponentLocation` (`self.B`))))))

(fn `GetDirection`
  (params (Player :type "Actor Object Reference"))
  (returns (Begin :type "Vector Structure") (End :type "Vector Structure"))
  (bind _returnvalue (`self.K2_GetActorLocation` Player))
  (bind _returnvalue_2 (`SceneComponent.K2_GetComponentLocation` (`self.A`)))
  (bind _returnvalue_3 (`SceneComponent.K2_GetComponentLocation` (`self.B`)))
  (if (< (`KismetMathLibrary.Vector_Distance` _returnvalue (`SceneComponent.K2_GetComponentLocation` (`self.A`))) (`KismetMathLibrary.Vector_Distance` _returnvalue (`SceneComponent.K2_GetComponentLocation` (`self.B`))))
    (return _returnvalue_2 _returnvalue_3)
    (else
      (return _returnvalue_3 _returnvalue_2))))

(fn `GetInputAction`
  (params (Role :type "/Game/DBDRemake/Common/ENUM_Role Enum" :default "NewEnumerator0"))
  (returns (Input :type "InputAction Object Reference"))
  (return "/Game/DBDRemake/Input/Actions/IA_Interact1.IA_Interact1"))

(fn `GetInteractionInput`
  (params (Role :type "/Game/DBDRemake/Common/ENUM_Role Enum" :default "NewEnumerator0"))
  (returns (Input :type String))
  (return "SPACE"))

(fn `GetInteractionText`
  (params (Role :type "/Game/DBDRemake/Common/ENUM_Role Enum" :default "NewEnumerator0"))
  (returns (Text :type String))
  (switch `/Game/DBDRemake/Common/ENUM_Role` Role
    (:`NewEnumerator0`
      (if (`self.IsDropped`)
        (return "TRAVERSER")
        (else
          (return "RENVERSER"))))
    (:`NewEnumerator1`
      (return "DÉTRUIRE"))))

(fn `UserConstructionScript`)