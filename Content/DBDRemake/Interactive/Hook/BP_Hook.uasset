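; BP_Hook is the interactable hook in a Dead by Daylight remake, where killers hang carried survivors and other survivors free them.
; Box overlap registers the hook with the player's BPCInteract component only when that role can act, and role-based getters supply input and French prompt text.
; On server interaction it delegates to the killer or survivor, with multicast events updating SurvivorHooked and that survivor's hooked state.
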(event `self.Box.OnComponentBeginOverlap`
  (params (OverlappedComponent :type "PrimitiveComponent Object Reference") (OtherActor :type "Actor Object Reference") (OtherComp :type "PrimitiveComponent Object Reference") (OtherBodyIndex :type Integer) (bFromSweep :type Boolean) (SweepResult :type "HitResult Structure (by ref)"))
  (`self.ActorOverlap` OtherActor))

(event `self.Box.OnComponentEndOverlap`
  (params (OverlappedComponent :type "PrimitiveComponent Object Reference") (OtherActor :type "Actor Object Reference") (OtherComp :type "PrimitiveComponent Object Reference") (OtherBodyIndex :type Integer))
  (bind _asbp_player (cast `/Game/DBDRemake/Common/BP_Player` OtherActor))
  (`/Game/DBDRemake/Interactive/BPC_Interact.InteractObjectEndOverlap` (`/Game/DBDRemake/Common/BP_Player.BPC_Interact` _asbp_player)))

(event `/Game/DBDRemake/Interactive/BPI_Interact.EndInteraction`
  (params (Player :type "/Game/DBDRemake/Common/BP_Player Object Reference") (`ServerInteract?` :type Boolean)))

(event `/Game/DBDRemake/Interactive/BPI_Interact.BeginInteraction`
  (params (Player :type "/Game/DBDRemake/Common/BP_Player Object Reference") (`ServerInteract?` :type Boolean))
  (if `ServerInteract?`
    (switch `/Game/DBDRemake/Common/ENUM_Role` (`/Game/DBDRemake/Common/BP_Player.PlayerRole` Player)
      (:`NewEnumerator0`
        (bind _asbp_survivor (cast `/Game/DBDRemake/Survivor/BP_Survivor` Player))
        (`self.SurvivorHooked`
          (:`then`
            (`/Game/DBDRemake/Survivor/BP_Survivor.UnhookSurvivor` _asbp_survivor self))
          (:`else`)))
      (:`NewEnumerator1`
        (bind _asbp_killer (cast `/Game/DBDRemake/Killer/BP_Killer` Player))
        (bind _survivorhold (`/Game/DBDRemake/Killer/BP_Killer.SurvivorHold` _asbp_killer)
          (:`then`
            (`self.MC_HookSurvivor` _survivorhold)
            (`/Game/DBDRemake/Killer/BP_Killer.HookSurvivor` _asbp_killer))
          (:`else`))))))

(event `MC_HookSurvivor`
  (params (SurvivorHooked :type "/Game/DBDRemake/Survivor/BP_Survivor Object Reference"))
  (bind _output_get (set `self.SurvivorHooked` SurvivorHooked))
  (`/Game/DBDRemake/Survivor/BP_Survivor.GetHooked` _output_get self))

(event `UnhookSurvivor`
  (`self.MC_UnhookSurvivor`))

(event `MC_UnhookSurvivor`
  (bind _survivorhooked (`self.SurvivorHooked`)
    (:`then`
      (`/Game/DBDRemake/Survivor/BP_Survivor.GetUnhooked` _survivorhooked)
      (set `self.SurvivorHooked` null))
    (:`else`)))

(fn `ActorOverlap`
  (params (Actor :type "Actor Object Reference"))
  (locals (BP_Player_Ref :type "/Game/DBDRemake/Common/BP_Player Object Reference") (BP_Killer_Ref :type "/Game/DBDRemake/Killer/BP_Killer Object Reference") (BP_Survivor_Ref :type "/Game/DBDRemake/Survivor/BP_Survivor Object Reference"))
  (bind _bp_player_ref (`local.BP_Player_Ref`))
  (bind _bp_player_ref_2 (`local.BP_Player_Ref`))
  (bind _asbp_player (cast `/Game/DBDRemake/Common/BP_Player` Actor))
  (bind _output_get (set `local.BP_Player_Ref` _asbp_player))
  (switch `/Game/DBDRemake/Common/ENUM_Role` (`/Game/DBDRemake/Common/BP_Player.PlayerRole` _output_get)
    (:`NewEnumerator0`
      (`/Engine/EditorBlueprintResources/StandardMacros.IsValid` (`self.SurvivorHooked`)
        (:`Is Valid`
          (bind _asbp_survivor (cast `/Game/DBDRemake/Survivor/BP_Survivor` (`local.BP_Player_Ref`)))
          (bind _output_get_2 (set `local.BP_Survivor_Ref` _asbp_survivor))
          (if (!= _output_get_2 (`self.SurvivorHooked`))
            (`/Game/DBDRemake/Interactive/BPC_Interact.InteractObjectBeginOverlap` (`/Game/DBDRemake/Common/BP_Player.BPC_Interact` _bp_player_ref) self _bp_player_ref)))))
    (:`NewEnumerator1`
      (`/Engine/EditorBlueprintResources/StandardMacros.IsValid` (`self.SurvivorHooked`)
        (:`Is Not Valid`
          (bind _asbp_killer (cast `/Game/DBDRemake/Killer/BP_Killer` (`local.BP_Player_Ref`)))
          (bind _output_get_3 (set `local.BP_Killer_Ref` _asbp_killer))
          (`/Game/DBDRemake/Killer/BP_Killer.SurvivorHold` _output_get_3
            (:`then`
              (`/Game/DBDRemake/Interactive/BPC_Interact.InteractObjectBeginOverlap` (`/Game/DBDRemake/Common/BP_Player.BPC_Interact` _bp_player_ref_2) self _bp_player_ref_2))
            (:`else`)))))))

(fn `GetInputAction`
  (params (Role :type "/Game/DBDRemake/Common/ENUM_Role Enum" :default "NewEnumerator0"))
  (returns (Input :type "InputAction Object Reference"))
  (switch `/Game/DBDRemake/Common/ENUM_Role` Role
    (:`NewEnumerator0`
      (return "/Game/DBDRemake/Input/Actions/IA_Interact2.IA_Interact2"))
    (:`NewEnumerator1`
      (return "/Game/DBDRemake/Input/Actions/IA_Interact1.IA_Interact1"))))

(fn `GetInteractionInput`
  (params (Role :type "/Game/DBDRemake/Common/ENUM_Role Enum" :default "NewEnumerator0"))
  (returns (Input :type String))
  (switch `/Game/DBDRemake/Common/ENUM_Role` Role
    (:`NewEnumerator0`
      (return "M1"))
    (:`NewEnumerator1`
      (return "SPACE"))))

(fn `GetInteractionText`
  (params (Role :type "/Game/DBDRemake/Common/ENUM_Role Enum" :default "NewEnumerator0"))
  (returns (Text :type String))
  (switch `/Game/DBDRemake/Common/ENUM_Role` Role
    (:`NewEnumerator0`
      (return "DÉCROCHER"))
    (:`NewEnumerator1`
      (return "ACCROCHER"))))

(fn `UserConstructionScript`)