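; BP_Exit is the exit trigger through which survivors escape a match.
; When a player with the Survivor role overlaps ExitBox, the authority calls MC_TeleportSurvivor, whose prefix suggests a multicast.
; That event moves the survivor to ExitPoint, sets HasEscaped and reports the escape to GS_DBDRemake through SurvivorEscape.
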(event `self.ExitBox.OnComponentBeginOverlap`
  (params (OverlappedComponent :type "PrimitiveComponent Object Reference") (OtherActor :type "Actor Object Reference") (OtherComp :type "PrimitiveComponent Object Reference") (OtherBodyIndex :type Integer) (bFromSweep :type Boolean) (SweepResult :type "HitResult Structure (by ref)"))
  (bind _asbp_player (cast `/Game/DBDRemake/Common/BP_Player` OtherActor))
  (switch `/Game/DBDRemake/Common/ENUM_Role` (`/Game/DBDRemake/Common/BP_Player.PlayerRole` _asbp_player)
    (:`NewEnumerator0`
      (bind _asbp_survivor (cast `/Game/DBDRemake/Survivor/BP_Survivor` _asbp_player))
      (`/Engine/EditorBlueprintResources/ActorMacros.Switch Has Authority`
        (:`Authority`
          (`self.MC_TeleportSurvivor` _asbp_survivor))))))

(event `MC_TeleportSurvivor`
  (params (Survivor :type "/Game/DBDRemake/Survivor/BP_Survivor Object Reference"))
  (`self.K2_SetActorLocation` Survivor (`SceneComponent.K2_GetComponentLocation` (`self.ExitPoint`)) false false)
  (set `/Game/DBDRemake/Survivor/BP_Survivor.HasEscaped` true Survivor)
  (bind _asgs_dbdremake (cast `/Game/DBDRemake/GS_DBDRemake` (`GameplayStatics.GetGameState`)))
  (`/Game/DBDRemake/GS_DBDRemake.SurvivorEscape` _asgs_dbdremake))

(fn `UserConstructionScript`)