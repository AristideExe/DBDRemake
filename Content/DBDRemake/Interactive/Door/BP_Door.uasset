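; Double door that survivors open by holding an interaction, likely an exit or gate in this DBD remake.
; Box overlap registers it with the survivor's interact component and adds a progress bar fed by the door's progress getters.
; A looping server timer accumulates progress while interaction lasts, keeping it when interrupted.
; At maximum, a multicast disables the box collision and plays a timeline sliding both panels apart.
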(event `self.Box.OnComponentBeginOverlap`
  (params (OverlappedComponent :type "PrimitiveComponent Object Reference") (OtherActor :type "Actor Object Reference") (OtherComp :type "PrimitiveComponent Object Reference") (OtherBodyIndex :type Integer) (bFromSweep :type Boolean) (SweepResult :type "HitResult Structure (by ref)"))
  (bind _asbp_survivor (cast `/Game/DBDRemake/Survivor/BP_Survivor` OtherActor))
  (switch `/Game/DBDRemake/Common/ENUM_Role` (`/Game/DBDRemake/Common/BP_Player.PlayerRole` _asbp_survivor)
    (:`NewEnumerator0`
      (if (`self.CanBeOpened`)
        (`/Game/DBDRemake/Interactive/BPC_Interact.InteractObjectBeginOverlap` (`/Game/DBDRemake/Common/BP_Player.BPC_Interact` _asbp_survivor) self _asbp_survivor)
        (bind _returnvalue (`|CreateWidget` "/Game/DBDRemake/UI/UI_ProgressBar.UI_ProgressBar_C" null self))
        (bind _output_get (set `self.ProgressBar` _returnvalue))
        (`/Game/DBDRemake/Common/BP_Player.AddProgressBar` _asbp_survivor _output_get)))))

(event `/Game/DBDRemake/Interactive/BPI_Interact.BeginInteraction`
  (params (Player :type "/Game/DBDRemake/Common/BP_Player Object Reference") (`ServerInteract?` :type Boolean))
  (if `ServerInteract?`
    (switch `/Game/DBDRemake/Common/ENUM_Role` (`/Game/DBDRemake/Common/BP_Player.PlayerRole` Player)
      (:`NewEnumerator0`
        (cast `/Game/DBDRemake/Survivor/BP_Survivor` Player)
        (`self.SR_OpenDoor`)))))

(event `SR_OpenDoor`
  (bind _returnvalue (`KismetSystemLibrary.K2_SetTimerDelegate` (delegate `OpenDoor`) 0.2 true))
  (set `self.OpenTimerHandle` _returnvalue))

(event `OpenDoor`
  (bind _output_get (set `self.OpenProgress` (+ (`self.OpenProgress`) (`self.OpenSpeed`))))
  (if (>= _output_get (`self.OpenMaxProgress`))
    (`KismetSystemLibrary.K2_ClearAndInvalidateTimerHandle` (`self.OpenTimerHandle`))
    (`self.MC_DoorOpening`)))

(event `MC_DoorOpening`
  (`PrimitiveComponent.SetCollisionEnabled` (`self.Box`) "NoCollision")
  (`Timeline|Door Opening` :!via `PlayFromStart`
    (:`Update`
      (`SceneComponent.K2_AddRelativeLocation` (`self.DoorLeft`) (-6.0 0.0 0.0) false false)
      (`SceneComponent.K2_AddRelativeLocation` (`self.DoorRight`) (6.0 0.0 0.0) false false))))

(event `/Game/DBDRemake/Interactive/BPI_Interact.EndInteraction`
  (params (Player :type "/Game/DBDRemake/Common/BP_Player Object Reference") (`ServerInteract?` :type Boolean))
  (if `ServerInteract?`
    (switch `/Game/DBDRemake/Common/ENUM_Role` (`/Game/DBDRemake/Common/BP_Player.PlayerRole` Player)
      (:`NewEnumerator0`
        (cast `/Game/DBDRemake/Survivor/BP_Survivor` Player)
        (`self.SR_StopOpening`)))))

(event `SR_StopOpening`
  (`KismetSystemLibrary.K2_ClearAndInvalidateTimerHandle` (`self.OpenTimerHandle`)))

(event `self.Box.OnComponentEndOverlap`
  (params (OverlappedComponent :type "PrimitiveComponent Object Reference") (OtherActor :type "Actor Object Reference") (OtherComp :type "PrimitiveComponent Object Reference") (OtherBodyIndex :type Integer))
  (bind _asbp_player (cast `/Game/DBDRemake/Common/BP_Player` OtherActor))
  (`/Game/DBDRemake/Interactive/BPC_Interact.InteractObjectEndOverlap` (`/Game/DBDRemake/Common/BP_Player.BPC_Interact` _asbp_player))
  (`/Game/DBDRemake/Common/BP_Player.RemoveProgressBar` _asbp_player (`self.ProgressBar`)))

(fn `CanBeOpened`
  (returns (CanBeOpened :type Boolean))
  (return true))

(fn `GetInputAction`
  (params (Role :type "/Game/DBDRemake/Common/ENUM_Role Enum" :default "NewEnumerator0"))
  (returns (Input :type "InputAction Object Reference"))
  (switch `/Game/DBDRemake/Common/ENUM_Role` Role
    (:`NewEnumerator0`
      (return "/Game/DBDRemake/Input/Actions/IA_Interact2.IA_Interact2"))))

(fn `GetInteractionInput`
  (params (Role :type "/Game/DBDRemake/Common/ENUM_Role Enum" :default "NewEnumerator0"))
  (returns (Input :type String))
  (switch `/Game/DBDRemake/Common/ENUM_Role` Role
    (:`NewEnumerator0`
      (return "M1"))))

(fn `GetInteractionText`
  (params (Role :type "/Game/DBDRemake/Common/ENUM_Role Enum" :default "NewEnumerator0"))
  (returns (Text :type String))
  (switch `/Game/DBDRemake/Common/ENUM_Role` Role
    (:`NewEnumerator0`
      (return "OUVRIR"))))

(fn `GetMaxProgress`
  (returns (MaxProgress :type "Float (double-precision)"))
  (return (`KismetMathLibrary.Conv_IntToDouble` (`self.OpenMaxProgress`))))

(fn `GetProgess`
  (returns (Progress :type "Float (double-precision)"))
  (return (`KismetMathLibrary.Conv_IntToDouble` (`self.OpenProgress`))))

(fn `UserConstructionScript`)