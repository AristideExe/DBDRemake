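; Generator objective for a Dead by Daylight remake that survivors repair and the killer can damage.
; Four trigger boxes register role-specific interactions and give each survivor a progress bar widget, fed by the generator's progress getters.
; Looping timers drive repair, scaled by repairer count, and regression after a break, using server and multicast-prefixed events.
; Completion disables the boxes' collision; the closest breaking point lookup is a zero-vector stub.
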(event `self.Box.OnComponentBeginOverlap`
  (params (OverlappedComponent :type "PrimitiveComponent Object Reference") (OtherActor :type "Actor Object Reference") (OtherComp :type "PrimitiveComponent Object Reference") (OtherBodyIndex :type Integer) (bFromSweep :type Boolean) (SweepResult :type "HitResult Structure (by ref)"))
  ;[0 0.1221 0.15 1 50] Actor Overlap
  (`self.ActorOverlap` OtherActor))

(event `self.Box.OnComponentEndOverlap`
  (params (OverlappedComponent :type "PrimitiveComponent Object Reference") (OtherActor :type "Actor Object Reference") (OtherComp :type "PrimitiveComponent Object Reference") (OtherBodyIndex :type Integer))
  ;[0 0.1221 0.15 1 50] Actor Overlap
  (`self.ActorEndOverlap` OtherActor))

(event `self.Box1.OnComponentEndOverlap`
  (params (OverlappedComponent :type "PrimitiveComponent Object Reference") (OtherActor :type "Actor Object Reference") (OtherComp :type "PrimitiveComponent Object Reference") (OtherBodyIndex :type Integer))
  ;[0 0.1221 0.15 1 50] Actor Overlap
  (`self.ActorEndOverlap` OtherActor))

(event `self.Box1.OnComponentBeginOverlap`
  (params (OverlappedComponent :type "PrimitiveComponent Object Reference") (OtherActor :type "Actor Object Reference") (OtherComp :type "PrimitiveComponent Object Reference") (OtherBodyIndex :type Integer) (bFromSweep :type Boolean) (SweepResult :type "HitResult Structure (by ref)"))
  ;[0 0.1221 0.15 1 50] Actor Overlap
  (`self.ActorOverlap` OtherActor))

(event `/Game/DBDRemake/Interactive/BPI_Interact.BeginInteraction`
  (params (Player :type "/Game/DBDRemake/Common/BP_Player Object Reference") (`ServerInteract?` :type Boolean))
  ;[0.06848 0.15 0.001214 1 50] Interaction
  (if `ServerInteract?`
    (switch `/Game/DBDRemake/Common/ENUM_Role` (`/Game/DBDRemake/Common/BP_Player.PlayerRole` Player)
      (:`NewEnumerator0`
        (bind _asbp_survivor (cast `/Game/DBDRemake/Survivor/BP_Survivor` Player))
        (`/Game/DBDRemake/Survivor/BP_Survivor.StartRepairing` _asbp_survivor)
        (`self.SR_RepairGenerator` _asbp_survivor))
      (:`NewEnumerator1`
        (bind _asbp_killer (cast `/Game/DBDRemake/Killer/BP_Killer` Player))
        (`/Game/DBDRemake/Killer/BP_Killer.DestroyGenerator` _asbp_killer self (`self.GetClosestBreakingPoint` _asbp_killer))))))

(event `self.Box2.OnComponentBeginOverlap`
  (params (OverlappedComponent :type "PrimitiveComponent Object Reference") (OtherActor :type "Actor Object Reference") (OtherComp :type "PrimitiveComponent Object Reference") (OtherBodyIndex :type Integer) (bFromSweep :type Boolean) (SweepResult :type "HitResult Structure (by ref)"))
  ;[0 0.1221 0.15 1 50] Actor Overlap
  (`self.ActorOverlap` OtherActor))

(event `self.Box2.OnComponentEndOverlap`
  (params (OverlappedComponent :type "PrimitiveComponent Object Reference") (OtherActor :type "Actor Object Reference") (OtherComp :type "PrimitiveComponent Object Reference") (OtherBodyIndex :type Integer))
  ;[0 0.1221 0.15 1 50] Actor Overlap
  (`self.ActorEndOverlap` OtherActor))

(event `self.Box3.OnComponentBeginOverlap`
  (params (OverlappedComponent :type "PrimitiveComponent Object Reference") (OtherActor :type "Actor Object Reference") (OtherComp :type "PrimitiveComponent Object Reference") (OtherBodyIndex :type Integer) (bFromSweep :type Boolean) (SweepResult :type "HitResult Structure (by ref)"))
  ;[0 0.1221 0.15 1 50] Actor Overlap
  (`self.ActorOverlap` OtherActor))

(event `self.Box3.OnComponentEndOverlap`
  (params (OverlappedComponent :type "PrimitiveComponent Object Reference") (OtherActor :type "Actor Object Reference") (OtherComp :type "PrimitiveComponent Object Reference") (OtherBodyIndex :type Integer))
  ;[0 0.1221 0.15 1 50] Actor Overlap
  (`self.ActorEndOverlap` OtherActor))

(event `/Game/DBDRemake/Interactive/BPI_Interact.EndInteraction`
  (params (Player :type "/Game/DBDRemake/Common/BP_Player Object Reference") (`ServerInteract?` :type Boolean))
  ;[0.06848 0.15 0.001214 1 50] End of Interaction
  (if `ServerInteract?`
    (switch `/Game/DBDRemake/Common/ENUM_Role` (`/Game/DBDRemake/Common/BP_Player.PlayerRole` Player)
      (:`NewEnumerator0`
        (bind _asbp_survivor (cast `/Game/DBDRemake/Survivor/BP_Survivor` Player))
        (`/Game/DBDRemake/Survivor/BP_Survivor.StopRepairing` _asbp_survivor)
        (`self.MC_SurvivorStopRepair`)))))

(event `BreakGenerator`
  ;[0.15 0.15 0.15 0.5 50] Break Generator
  (`self.SR_BreakGenerator`))

(event `SR_RepairGenerator`
  (params (Player :type "/Game/DBDRemake/Survivor/BP_Survivor Object Reference"))
  ;[0.15 0.15 0.15 0.5 50] Repairing
  (if (`.ReturnValue` (`BlueprintMapLibrary.Map_Find` (`self.SurvivorRepairingProgressBars`) Player))
    (`/Engine/EditorBlueprintResources/StandardMacros.IncrementInt` (`self.NumberOfPlayersRepairing`)
      (:`  `
        (`KismetSystemLibrary.K2_ClearAndInvalidateTimerHandle` (`self.RegressionTimerHandle`))
        (if (not (`self.IsBeingRepaired?`))
          (set `self.IsBeingRepaired?` true)
          (bind _returnvalue (`KismetSystemLibrary.K2_SetTimerDelegate` (delegate `RepairGenerator`) 0.2 true))
          (set `self.RepairTimerHandle` _returnvalue))))))

(event `SR_BreakGenerator`
  ;[0.15 0.15 0.15 0.5 50] Break Generator
  (set `self.RepairProgress` (`KismetMathLibrary.Clamp` (- (`self.RepairProgress`) (`self.BreakingMalus`)) 0 (`self.RepairMaxProgress`)))
  (bind _returnvalue (`KismetSystemLibrary.K2_SetTimerDelegate` (delegate `RegressGenerator`) 0.2 true))
  (set `self.RegressionTimerHandle` _returnvalue))

(event `RegressGenerator`
  ;[0.15 0.15 0.15 0.5 50] Break Generator
  (set `self.RepairProgress` (`KismetMathLibrary.Clamp` (- (`self.RepairProgress`) (`self.RegressionSpeed`)) 0 (`self.RepairMaxProgress`))))

(event `RepairGenerator`
  ;[0.15 0.15 0.15 0.5 50] Repairing
  (set `self.RepairProgress` (+ (`self.RepairProgress`) (* (`self.RepairSpeed`) (`self.NumberOfPlayersRepairing`))))
  (if (`self.IsGeneratorFinished?`)
    (`KismetSystemLibrary.K2_ClearAndInvalidateTimerHandle` (`self.RepairTimerHandle`))
    (`self.MC_RemoveBoxesCollision`)))

(event `MC_SurvivorStopRepair`
  (`/Engine/EditorBlueprintResources/StandardMacros.DecrementInt` (`self.NumberOfPlayersRepairing`)))

(event `self.ReceiveBeginPlay`
  (bind _asui_generator_progress (cast `/Game/DBDRemake/UI/UI_GeneratorProgress` (`WidgetComponent.GetWidget` (`self.ProgressBar`))))
  (set `/Game/DBDRemake/UI/UI_GeneratorProgress.BPI_ProgressBar` self _asui_generator_progress))

(event `MC_RemoveBoxesCollision`
  (for _array_element (`|MakeArray` (`self.Box`) (`self.Box1`) (`self.Box2`) (`self.Box3`))
    (`PrimitiveComponent.SetCollisionEnabled` _array_element "NoCollision")))

(fn `ActorEndOverlap`
  (params (Actor :type "Actor Object Reference"))
  (bind _asbp_player (cast `/Game/DBDRemake/Common/BP_Player` Actor))
  (`/Game/DBDRemake/Interactive/BPC_Interact.InteractObjectEndOverlap` (`/Game/DBDRemake/Common/BP_Player.BPC_Interact` _asbp_player))
  (switch `/Game/DBDRemake/Common/ENUM_Role` (`/Game/DBDRemake/Common/BP_Player.PlayerRole` _asbp_player)
    (:`NewEnumerator0`
      (bind _asbp_survivor (cast `/Game/DBDRemake/Survivor/BP_Survivor` _asbp_player))
      (bind (_value _returnvalue) (`BlueprintMapLibrary.Map_Find` (`self.SurvivorRepairingProgressBars`) _asbp_survivor))
      (if _returnvalue
        (`/Game/DBDRemake/Common/BP_Player.RemoveProgressBar` _asbp_survivor _value)
        (`/Game/DBDRemake/Survivor/BP_Survivor.StopRepairing` _asbp_survivor)
        (`BlueprintMapLibrary.Map_Remove` (`self.SurvivorRepairingProgressBars`) _asbp_survivor)))))

(fn `ActorOverlap`
  (params (Actor :type "Actor Object Reference"))
  (locals (BPC_Interact_Ref :type "/Game/DBDRemake/Interactive/BPC_Interact Object Reference") (BP_Player_Ref :type "/Game/DBDRemake/Common/BP_Player Object Reference") (BP_Survivor_Ref :type "/Game/DBDRemake/Survivor/BP_Survivor Object Reference"))
  (bind _bp_survivor_ref (`local.BP_Survivor_Ref`))
  (bind _asbp_player (cast `/Game/DBDRemake/Common/BP_Player` Actor))
  (bind _output_get (set `local.BP_Player_Ref` _asbp_player))
  (set `local.BPC_Interact_Ref` (`/Game/DBDRemake/Common/BP_Player.BPC_Interact` _output_get))
  (switch `/Game/DBDRemake/Common/ENUM_Role` (`/Game/DBDRemake/Common/BP_Player.PlayerRole` (`local.BP_Player_Ref`))
    (:`NewEnumerator0`
      (if (not (`self.IsGeneratorFinished?`))
        (bind _asbp_survivor (cast `/Game/DBDRemake/Survivor/BP_Survivor` (`local.BP_Player_Ref`)))
        (bind _output_get_2 (set `local.BP_Survivor_Ref` _asbp_survivor))
        (if (not (`/Game/DBDRemake/Survivor/BP_Survivor.IsCrawling` _output_get_2))
          (`/Game/DBDRemake/Interactive/BPC_Interact.InteractObjectBeginOverlap` (`local.BPC_Interact_Ref`) self (`local.BP_Player_Ref`)))
        (bind _returnvalue (`|CreateWidget` "/Game/DBDRemake/UI/UI_ProgressBar.UI_ProgressBar_C" null self))
        (`BlueprintMapLibrary.Map_Add` (`self.SurvivorRepairingProgressBars`) _bp_survivor_ref _returnvalue)
        (`/Game/DBDRemake/Common/BP_Player.AddProgressBar` _bp_survivor_ref _returnvalue)))
    (:`NewEnumerator1`
      (if (and (> (`self.RepairProgress`) 0) (not (`self.IsGeneratorFinished?`)))
        (`/Game/DBDRemake/Interactive/BPC_Interact.InteractObjectBeginOverlap` (`local.BPC_Interact_Ref`) self (`local.BP_Player_Ref`))))))

(fn `GetClosestBreakingPoint`
  (params (Player :type "Actor Object Reference"))
  (returns (ClosetPoint :type "Vector Structure"))
  (return (0.0 0.0 0.0)))

(fn `GetInputAction`
  (params (Role :type "/Game/DBDRemake/Common/ENUM_Role Enum" :default "NewEnumerator0"))
  (returns (Input :type "InputAction Object Reference"))
  (switch `/Game/DBDRemake/Common/ENUM_Role` Role
    (:`NewEnumerator0`
      (return "/Game/DBDRemake/Input/Actions/IA_Interact2.IA_Interact2"))
    (:`NewEnumerator1`
      (return "/Game/DBDRemake/Input/Actions/IA_Interact1.IA_Interact1"))))

(fn `GetInteractionInput`
  (params (Role :type "/Game/DBDRemake/Common/ENUM_Role Enum" :default "NewEnumerator0"))
  (returns (Input :type String))
  (switch `/Game/DBDRemake/Common/ENUM_Role` Role
    (:`NewEnumerator0`
      (return "M1"))
    (:`NewEnumerator1`
      (return "SPACE"))))

(fn `GetInteractionText`
  (params (Role :type "/Game/DBDRemake/Common/ENUM_Role Enum" :default "NewEnumerator0"))
  (returns (Text :type String))
  (switch `/Game/DBDRemake/Common/ENUM_Role` Role
    (:`NewEnumerator0`
      (return "RÉPARER"))
    (:`NewEnumerator1`
      (return "DÉTRUIRE"))))

(fn `GetMaxProgress`
  (returns (MaxProgress :type "Float (double-precision)"))
  (return (`KismetMathLibrary.Conv_IntToDouble` (`self.RepairMaxProgress`))))

(fn `GetProgess`
  (returns (Progress :type "Float (double-precision)"))
  (return (`KismetMathLibrary.Conv_IntToDouble` (`self.RepairProgress`))))

(fn `IsGeneratorFinished?`
  (returns (Finished :type Boolean))
  (return (>= (`self.RepairProgress`) (`self.RepairMaxProgress`))))

(fn `UserConstructionScript`)