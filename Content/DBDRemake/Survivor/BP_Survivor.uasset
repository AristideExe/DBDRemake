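; Survivor character for a Dead by Daylight remake, handling sprint, crouch, repair, vaults and the injury-to-hook flow.
; Movement changes apply locally and through SR_ server events; windows and pallets use montages with timeline location lerps.
; Damage steps health from healthy through injured to dying crawl, with capsule collision disabled.
; An overlap box offers crawling survivors to the killer's interact component for pickup, then multicast events attach them to killer or hook.
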(event `StartSprinting`
  ;[0.15 0.09759 0 0.502 50] Sprint
  (if (`self.IsCrawling`)
    _
    (elif (not (`self.IsPressingCrouch?`))
      (set `CharacterMovementComponent.MaxWalkSpeed` (`self.SprintSpeed`) (`self.CharacterMovement`))
      (`self.SR_StartSprinting`))))

(event `SR_StartSprinting`
  ;[0.15 0.09759 0 0.502 50] Sprint
  (set `CharacterMovementComponent.MaxWalkSpeed` (`self.SprintSpeed`) (`self.CharacterMovement`)))

(event `EnhancedInput|/Game/DBDRemake/Input/Actions/IA_Sprint`
  (params (ActionValue :type Boolean) (ElapsedSeconds :type "Float (double-precision)") (TriggeredSeconds :type "Float (double-precision)") (InputAction :type "InputAction Object Reference" :default "/Game/DBDRemake/Input/Actions/IA_Sprint.IA_Sprint"))
  ;[0.15 0.09759 0 0.502 50] Sprint
  (:`Started`
    (set `self.IsPressingSprint?` true)
    (`self.StartSprinting`))
  (:`Canceled`
    (set `self.IsPressingSprint?` false :!label _label)
    (`self.StopSprinting`))
  (:`Completed`
    (goto _label)))

(event `StopSprinting`
  ;[0.15 0.09759 0 0.502 50] Sprint
  (if (`self.IsCrawling`)
    _
    (elif (not (`self.IsPressingCrouch?`))
      (set `CharacterMovementComponent.MaxWalkSpeed` (`self.WalkSpeed`) (`self.CharacterMovement`))
      (`self.SR_StopSprinting`))))

(event `SR_StopSprinting`
  ;[0.15 0.09759 0 0.502 50] Sprint
  (set `CharacterMovementComponent.MaxWalkSpeed` (`self.WalkSpeed`) (`self.CharacterMovement`)))

(event `StartCrouching`
  ;[0.15 0.09759 0 0.502 50] Crouching
  (if (not (`self.IsCrawling`))
    (set `CharacterMovementComponent.MaxWalkSpeed` (`self.CrouchSpeed`) (`self.CharacterMovement`))
    (`self.SR_StartCrouching`)))

(event `StartRepairing`
  ;[0.000662 0.06771 0.15 0.5 50] Repairing
  (`self.SR_StartRepairing`))

(event `SR_StartRepairing`
  ;[0.000662 0.06771 0.15 0.5 50] Repairing
  (`CharacterMovementComponent.DisableMovement` (`self.CharacterMovement`))
  (set `self.IsRepairing?` true))

(event `SR_StartCrouching`
  ;[0.15 0.09759 0 0.502 50] Crouching
  (set `CharacterMovementComponent.MaxWalkSpeed` (`self.CrouchSpeed`) (`self.CharacterMovement`))
  (set `self.IsCrouching` true))

(event `EnhancedInput|/Game/DBDRemake/Input/Actions/IA_Crouch`
  (params (ActionValue :type Boolean) (ElapsedSeconds :type "Float (double-precision)") (TriggeredSeconds :type "Float (double-precision)") (InputAction :type "InputAction Object Reference" :default "/Game/DBDRemake/Input/Actions/IA_Crouch.IA_Crouch"))
  ;[0.15 0.09759 0 0.502 50] Crouching
  (:`Started`
    (set `self.IsPressingCrouch?` true)
    (`self.StartCrouching`))
  (:`Canceled`
    (set `self.IsPressingCrouch?` false :!label _label_2)
    (`self.StopCrouching`))
  (:`Completed`
    (goto _label_2)))

(event `StopRepairing`
  ;[0.000662 0.06771 0.15 0.5 50] Repairing
  (`self.SR_StopRepairing`))

(event `StopCrouching`
  ;[0.15 0.09759 0 0.502 50] Crouching
  (if (`self.IsCrawling`)
    _
    (elif (`self.IsPressingSprint?`)
      (`self.StartSprinting`)
      (else
        (set `CharacterMovementComponent.MaxWalkSpeed` (`self.WalkSpeed`) (`self.CharacterMovement`))
        (`self.SR_StopCrouching`)))))

(event `SR_StopRepairing`
  ;[0.000662 0.06771 0.15 0.5 50] Repairing
  (`CharacterMovementComponent.SetMovementMode` (`self.CharacterMovement`) "MOVE_Walking" 0)
  (set `self.IsRepairing?` false))

(event `SR_StopCrouching`
  ;[0.15 0.09759 0 0.502 50] Crouching
  (set `CharacterMovementComponent.MaxWalkSpeed` (`self.WalkSpeed`) (`self.CharacterMovement`))
  (set `self.IsCrouching` false))

(event `GoThroughWindow`
  (params (Start :type "Vector Structure") (End :type "Vector Structure"))
  ;[0.1441 0 0.15 0.502 50] Go Through Window
  (`/Engine/EditorBlueprintResources/ActorMacros.Switch Has Authority`
    (:`Authority`
      (`self.SR_GoThroughWindow` Start End))))

(event `SR_GoThroughWindow`
  (params (Start :type "Vector Structure") (End :type "Vector Structure"))
  ;[0.1441 0 0.15 0.502 50] Go Through Window
  (`CharacterMovementComponent.DisableMovement` (`self.CharacterMovement`))
  (`|PlayMontage` (`self.Mesh`) "/Game/Characters/Mannequins/Anims/Unarmed/Jump_Montage.Jump_Montage"
    (:`then`
      (bind (_direction _alpha) (`Timeline|GoThroughWindowTimeline` :!via `PlayFromStart`)
        (:`Update`
          (`self.K2_SetActorLocation` (`KismetMathLibrary.VLerp` Start End _alpha)))
        (:`Finished`
          (`CharacterMovementComponent.SetMovementMode` (`self.CharacterMovement`) "MOVE_Walking" 0))))))

(event `TakeDamage`
  ;[0.15 0.005942 0 0.5 50] Take Damage
  (`self.SR_TakeDamage`))

(event `SR_TakeDamage`
  ;[0.15 0.005942 0 0.5 50] Take Damage
  (switch `/Game/DBDRemake/Survivor/ENUM_HealthState` (`self.HealthState`)
    (:`NewEnumerator0`
      (bind _output_get (set `self.HealthState` "NewEnumerator1"))
      (`KismetSystemLibrary.PrintString` (`|GetEnumeratorNameAsString` _output_get)))
    (:`NewEnumerator1`
      (set `self.HealthState` "NewEnumerator2")
      (`self.MC_GetDown`))))

(event `VaultPallet`
  (params (Start :type "Vector Structure") (End :type "Vector Structure"))
  ;[0.1441 0 0.15 0.502 50] Vault Pallet
  (`/Engine/EditorBlueprintResources/ActorMacros.Switch Has Authority`
    (:`Authority`
      (`self.SR_VaultPallet` Start End))))

(event `SR_VaultPallet`
  (params (Start :type "Vector Structure") (End :type "Vector Structure"))
  ;[0.1441 0 0.15 0.502 50] Vault Pallet
  (`CharacterMovementComponent.DisableMovement` (`self.CharacterMovement`))
  (`|PlayMontage` (`self.Mesh`) "/Game/Characters/Mannequins/Anims/Unarmed/Jump_Montage.Jump_Montage"
    (:`then`
      (bind (_direction _alpha) (`Timeline|VaultPalletTimeline` :!via `PlayFromStart`)
        (:`Update`
          (`self.K2_SetActorLocation` (`KismetMathLibrary.VLerp` Start End _alpha)))
        (:`Finished`
          (`CharacterMovementComponent.SetMovementMode` (`self.CharacterMovement`) "MOVE_Walking" 0))))))

(event `MC_GetDown`
  (set `CharacterMovementComponent.MaxWalkSpeed` (`self.DyingWalkSped`) (`self.CharacterMovement`))
  (`self.RetrigerCollisions`)
  (`KismetSystemLibrary.Delay` 0.1)
  (`PrimitiveComponent.SetCollisionEnabled` (`self.CapsuleComponent`) "NoCollision") ; Disable collisions of player to be able to walk on it
)

(event `BeginGettingPickedUp`
  (params (Killer :type "/Game/DBDRemake/Killer/BP_Killer Object Reference"))
  (`self.MC_BeginGettingPickedUp` Killer))

(event `MC_BeginGettingPickedUp`
  (params (Killer :type "/Game/DBDRemake/Killer/BP_Killer Object Reference"))
  (`CharacterMovementComponent.DisableMovement` (`self.CharacterMovement`))
  (`self.K2_AttachToActor` Killer "hand_lSocket" "KeepWorld" "KeepRelative" "KeepRelative" true)
  (`/Game/DBDRemake/Interactive/BPC_Interact.InteractObjectEndOverlap` (`/Game/DBDRemake/Common/BP_Player.BPC_Interact` Killer)))

(event `self.Box.OnComponentBeginOverlap`
  (params (OverlappedComponent :type "PrimitiveComponent Object Reference") (OtherActor :type "Actor Object Reference") (OtherComp :type "PrimitiveComponent Object Reference") (OtherBodyIndex :type Integer) (bFromSweep :type Boolean) (SweepResult :type "HitResult Structure (by ref)"))
  (`self.ActorBeginOverlap` OtherActor))

(event `GetHooked`
  (params (Hook :type "/Game/DBDRemake/Interactive/Hook/BP_Hook Object Reference"))
  (`self.MC_GetHooked` Hook))

(event `self.Box.OnComponentEndOverlap`
  (params (OverlappedComponent :type "PrimitiveComponent Object Reference") (OtherActor :type "Actor Object Reference") (OtherComp :type "PrimitiveComponent Object Reference") (OtherBodyIndex :type Integer))
  (bind _asbp_player (cast `/Game/DBDRemake/Common/BP_Player` OtherActor))
  (`/Game/DBDRemake/Interactive/BPC_Interact.InteractObjectEndOverlap` (`/Game/DBDRemake/Common/BP_Player.BPC_Interact` _asbp_player)))

(event `MC_GetHooked`
  (params (Hook :type "/Game/DBDRemake/Interactive/Hook/BP_Hook Object Reference"))
  (bind _hookposition (`/Game/DBDRemake/Interactive/Hook/BP_Hook.HookPosition` Hook))
  (`self.K2_DetachFromActor` "KeepRelative")
  (`self.K2_SetActorLocation` (`SceneComponent.K2_GetComponentLocation` _hookposition))
  (`self.K2_SetActorRotation` (`SceneComponent.K2_GetComponentRotation` _hookposition))
  (`self.K2_AttachToActor` Hook "None" "KeepWorld" "KeepWorld" "KeepRelative")
  (set `self.IsHooked?` true))

(event `GetPickedUp`)

(event `/Game/DBDRemake/Interactive/BPI_Interact.BeginInteraction`
  (params (Player :type "/Game/DBDRemake/Common/BP_Player Object Reference") (`ServerInteract?` :type Boolean))
  (if `ServerInteract?`
    (switch `/Game/DBDRemake/Common/ENUM_Role` (`/Game/DBDRemake/Common/BP_Player.PlayerRole` Player)
      (:`NewEnumerator1`
        (bind _asbp_killer (cast `/Game/DBDRemake/Killer/BP_Killer` Player))
        (`/Game/DBDRemake/Killer/BP_Killer.PickUpSurvivor` _asbp_killer self)))))

(event `MC_GetPickedUp`)

(fn `ActorBeginOverlap`
  (params (Actor :type "Actor Object Reference"))
  (locals (BP_Player_Ref :type "/Game/DBDRemake/Common/BP_Player Object Reference"))
  (bind _bp_player_ref (`local.BP_Player_Ref`))
  (bind _asbp_player (cast `/Game/DBDRemake/Common/BP_Player` Actor))
  (bind _output_get (set `local.BP_Player_Ref` _asbp_player))
  (switch `/Game/DBDRemake/Common/ENUM_Role` (`/Game/DBDRemake/Common/BP_Player.PlayerRole` _output_get)
    (:`NewEnumerator1`
      (if (`self.IsCrawling`)
        (`/Game/DBDRemake/Interactive/BPC_Interact.InteractObjectBeginOverlap` (`/Game/DBDRemake/Common/BP_Player.BPC_Interact` _bp_player_ref) self _bp_player_ref)))))

(fn `GetInputAction`
  (params (Role :type "/Game/DBDRemake/Common/ENUM_Role Enum" :default "NewEnumerator0"))
  (returns (Input :type "InputAction Object Reference"))
  (switch `/Game/DBDRemake/Common/ENUM_Role` Role
    (:`NewEnumerator0`
      (return "/Game/DBDRemake/Input/Actions/IA_Interact2.IA_Interact2"))
    (:`NewEnumerator1`
      (return "/Game/DBDRemake/Input/Actions/IA_Interact1.IA_Interact1"))))

(fn `GetInteractionInput`
  (params (Role :type "/Game/DBDRemake/Common/ENUM_Role Enum" :default "NewEnumerator0"))
  (returns (Input :type String))
  (switch `/Game/DBDRemake/Common/ENUM_Role` Role
    (:`NewEnumerator0`
      (return "M1"))
    (:`NewEnumerator1`
      (return "SPACE"))))

(fn `GetInteractionText`
  (params (Role :type "/Game/DBDRemake/Common/ENUM_Role Enum" :default "NewEnumerator0"))
  (returns (Text :type String))
  (switch `/Game/DBDRemake/Common/ENUM_Role` Role
    (:`NewEnumerator0`
      (return "SOIGNER"))
    (:`NewEnumerator1`
      (return "RAMASSER"))))

(fn `IsCrawling`
  (returns (Crawling :type Boolean))
  (return (and (`|EnumEquality` (`self.HealthState`) "NewEnumerator2") (not (`self.IsHooked?`)))))

(fn `UserConstructionScript`)