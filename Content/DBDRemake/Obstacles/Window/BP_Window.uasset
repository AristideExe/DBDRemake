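; BP_Window is an interactable window obstacle that survivors can vault through.
; Box overlaps register or clear the window on the BPCInteractIcon of survivors and killers, with getters supplying the input action, key label and "TRAVERSER" text.
; Interact acts only for survivors, calling GoThroughWindow with start and end points from GetDirection.
; GetDirection starts from whichever of markers A or B is nearer the player, so traversal works from both sides.
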(event `self.Box.OnComponentBeginOverlap`
  (params (OverlappedComponent :type "PrimitiveComponent Object Reference") (OtherActor :type "Actor Object Reference") (OtherComp :type "PrimitiveComponent Object Reference") (OtherBodyIndex :type Integer) (bFromSweep :type Boolean) (SweepResult :type "HitResult Structure (by ref)"))
  (bind _asbp_survivor (cast `/Game/DBDRemake/Survivor/BP_Survivor` OtherActor)
    (:`then`
      (`/Game/DBDRemake/Common/BPC_InteractIcon.InteractObjectBeginOverlap` (`/Game/DBDRemake/Survivor/BP_Survivor.BPC_InteractIcon` _asbp_survivor) self _asbp_survivor))
    (:`CastFailed`
      (bind _asbp_killer (cast `/Game/DBDRemake/Killer/BP_Killer` OtherActor))
      (`/Game/DBDRemake/Common/BPC_InteractIcon.InteractObjectBeginOverlap` (`/Game/DBDRemake/Killer/BP_Killer.BPC_InteractIcon` _asbp_killer) self _asbp_killer))))

(event `self.Box.OnComponentEndOverlap`
  (params (OverlappedComponent :type "PrimitiveComponent Object Reference") (OtherActor :type "Actor Object Reference") (OtherComp :type "PrimitiveComponent Object Reference") (OtherBodyIndex :type Integer))
  (bind _asbp_survivor (cast `/Game/DBDRemake/Survivor/BP_Survivor` OtherActor)
    (:`then`
      (`/Game/DBDRemake/Common/BPC_InteractIcon.InteractObjectEndOverlap` (`/Game/DBDRemake/Survivor/BP_Survivor.BPC_InteractIcon` _asbp_survivor)))
    (:`CastFailed`
      (bind _asbp_killer (cast `/Game/DBDRemake/Killer/BP_Killer` OtherActor))
      (`/Game/DBDRemake/Common/BPC_InteractIcon.InteractObjectEndOverlap` (`/Game/DBDRemake/Killer/BP_Killer.BPC_InteractIcon` _asbp_killer)))))

(event `/Game/DBDRemake/Common/BPI_Interact.Interact`
  (params (Player :type "Actor Object Reference") (`ServerInteract?` :type Boolean))
  (bind _asbp_survivor (cast `/Game/DBDRemake/Survivor/BP_Survivor` Player))
  (bind (_begin _end) (`self.GetDirection` _asbp_survivor))
  (`/Game/DBDRemake/Survivor/BP_Survivor.GoThroughWindow` _asbp_survivor _begin _end))

(fn `GetDirection`
  (params (Player :type "Actor Object Reference"))
  (returns (Begin :type "Vector Structure") (End :type "Vector Structure"))
  (bind _returnvalue (`self.K2_GetActorLocation` Player))
  (bind _returnvalue_2 (`SceneComponent.K2_GetComponentLocation` (`self.A`)))
  (bind _returnvalue_3 (`SceneComponent.K2_GetComponentLocation` (`self.B`)))
  (if (< (`KismetMathLibrary.Vector_Distance` _returnvalue (`SceneComponent.K2_GetComponentLocation` (`self.A`))) (`KismetMathLibrary.Vector_Distance` _returnvalue (`SceneComponent.K2_GetComponentLocation` (`self.B`))))
    (return _returnvalue_2 _returnvalue_3)
    (else
      (return _returnvalue_3 _returnvalue_2))))

(fn `GetInputAction`
  (returns (Input :type "InputAction Object Reference"))
  (return "/Game/DBDRemake/Input/Actions/IA_Interact1.IA_Interact1"))

(fn `GetInteractionInput`
  (returns (Input :type String))
  (return "SPACE"))

(fn `GetInteractionText`
  (returns (Text :type String))
  (return "TRAVERSER"))

(fn `UserConstructionScript`)