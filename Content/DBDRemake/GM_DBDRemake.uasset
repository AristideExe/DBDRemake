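; Game mode for the DBD remake that assigns joining players to killer or survivor pawns.
; It tracks player controllers on login and logout, and once two or more are present, each login triggers a short delay, then respawns everyone.
; Spawning destroys any current pawn, gives the local (host) controller the killer and remote ones survivors, each at a randomly picked PlayerStart, with no check for reuse.
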(event `self.K2_PostLogin`
  (params (NewPlayer :type "PlayerController Object Reference"))
  (bind _players (`self.Players`))
  (`KismetArrayLibrary.Array_Add` _players NewPlayer)
  (if (>= (`KismetArrayLibrary.Array_Length` _players) 2)
    (`KismetSystemLibrary.Delay` 0.2)
    (for _array_element (`self.Players`)
      (`self.SpawnPlayer` _array_element))))

(event `self.K2_OnLogout`
  (params (ExitingController :type "Controller Object Reference"))
  (bind _asplayer_controller (cast `PlayerController` ExitingController))
  (`KismetArrayLibrary.Array_RemoveItem` (`self.Players`) _asplayer_controller))

(fn `FindRandomPlayerStart`
  (returns (PlayerStartTransform :type "Transform Structure"))
  (bind _outactors (`GameplayStatics.GetAllActorsOfClass` "/Script/Engine.PlayerStart"))
  (return (`self.GetTransform` (`|GetArrayItem` _outactors (`KismetMathLibrary.RandomIntegerInRange` 0 (- (`KismetArrayLibrary.Array_Length` _outactors) 1))))))

(fn `SpawnPlayer`
  (params (PlayerController :type "PlayerController Object Reference"))
  (bind _returnvalue (`Controller.K2_GetPawn` PlayerController))
  (bind _playerstarttransform (`self.FindRandomPlayerStart`))
  (`/Engine/EditorBlueprintResources/StandardMacros.IsValid` _returnvalue
    (:`Is Valid`
      (`self.K2_DestroyActor` _returnvalue))
    (:`Is Not Valid`
      _))
  (if (`Controller.IsLocalController` PlayerController)
    (bind _returnvalue_2 (`|SpawnActorFromClass` "/Game/DBDRemake/Killer/BP_Killer.BP_Killer_C" _playerstarttransform "Undefined" "MultiplyWithRoot" null null))
    (`Controller.Possess` PlayerController _returnvalue_2)
    (else
      (bind _returnvalue_3 (`|SpawnActorFromClass` "/Game/DBDRemake/Survivor/BP_Survivor.BP_Survivor_C" _playerstarttransform "Undefined" "MultiplyWithRoot" null null))
      (`Controller.Possess` PlayerController _returnvalue_3))))

(fn `UserConstructionScript`)