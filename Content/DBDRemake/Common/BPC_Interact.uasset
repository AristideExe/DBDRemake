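; Player interaction component for BP_Player that lets the player begin and end interactions with nearby objects through two input actions.
; Overlap functions store the interface-based target for the locally controlled pawn and show or hide its role-specific prompt in UI_Interact.
; Input counts only if it matches the action the target returns for the player's Role.
; Begin and end run locally first, then repeat through SR events with ServerInteract set true.
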(event `EnhancedInput|/Game/DBDRemake/Input/Actions/IA_Interact1`
  (params (ActionValue :type Boolean) (ElapsedSeconds :type "Float (double-precision)") (TriggeredSeconds :type "Float (double-precision)") (InputAction :type "InputAction Object Reference" :default "/Game/DBDRemake/Input/Actions/IA_Interact1.IA_Interact1"))
  (:`Started`
    (`self.StartInteractInput` InputAction))
  (:`Canceled`
    (`self.EndInteractInput` InputAction :!label _label))
  (:`Completed`
    (goto _label)))

(event `StartInteractInput`
  (params (Input :type "InputAction Object Reference"))
  (bind _interactobject (`self.InteractObject`))
  (bind _interactobject_2 (`self.InteractObject`))
  (if (`KismetSystemLibrary.IsValidInterface` _interactobject_2)
    (bind _input (`/Game/DBDRemake/Common/BPI_Interact.GetInputAction` _interactobject_2 (`self.Role`)))
    (if (== _input Input)
      (bind _asbp_player (cast `/Game/DBDRemake/Common/BP_Player` (`self.GetOwner`)))
      (`/Game/DBDRemake/Common/BPI_Interact.BeginInteraction` _interactobject _asbp_player false)
      (`self.SR_Interact` _interactobject _asbp_player))))

(event `EnhancedInput|/Game/DBDRemake/Input/Actions/IA_Interact2`
  (params (ActionValue :type Boolean) (ElapsedSeconds :type "Float (double-precision)") (TriggeredSeconds :type "Float (double-precision)") (InputAction :type "InputAction Object Reference" :default "/Game/DBDRemake/Input/Actions/IA_Interact2.IA_Interact2"))
  (:`Started`
    (`self.StartInteractInput` InputAction))
  (:`Canceled`
    (`self.EndInteractInput` InputAction :!label _label_2))
  (:`Completed`
    (goto _label_2)))

(event `EndInteractInput`
  (params (Input :type "InputAction Object Reference"))
  (bind _interactobject (`self.InteractObject`))
  (bind _interactobject_2 (`self.InteractObject`))
  (if (`KismetSystemLibrary.IsValidInterface` _interactobject_2)
    (bind _input (`/Game/DBDRemake/Common/BPI_Interact.GetInputAction` _interactobject_2 (`self.Role`)))
    (if (== _input Input)
      (bind _asbp_player (cast `/Game/DBDRemake/Common/BP_Player` (`self.GetOwner`)))
      (`/Game/DBDRemake/Common/BPI_Interact.EndInteraction` _interactobject _asbp_player false)
      (`self.SR_EndInteraction` _interactobject _asbp_player))))

(event `self.ReceiveBeginPlay`
  (bind _foundwidgets (`WidgetBlueprintLibrary.GetAllWidgetsOfClass` "/Game/DBDRemake/UI/UI_Interact.UI_Interact_C" false))
  (set `self.UI_Interact_Ref` (`|GetArrayItem` _foundwidgets)))

(event `SR_Interact`
  (params (Target :type "/Game/DBDRemake/Common/BPI_Interact Interface") (Player :type "/Game/DBDRemake/Common/BP_Player Object Reference"))
  (`/Game/DBDRemake/Common/BPI_Interact.BeginInteraction` Target Player true))

(event `SR_EndInteraction`
  (params (Target :type "/Game/DBDRemake/Common/BPI_Interact Interface") (Player :type "/Game/DBDRemake/Common/BP_Player Object Reference"))
  (`/Game/DBDRemake/Common/BPI_Interact.EndInteraction` Target Player true))

(fn `InteractObjectBeginOverlap`
  (params (Object :type "/Game/DBDRemake/Common/BPI_Interact Interface") (Pawn :type "Pawn Object Reference"))
  (bind _role (`self.Role`))
  (if (== Pawn (`Controller.K2_GetPawn` (`GameplayStatics.GetPlayerController` 0)))
    (bind _output_get (set `self.InteractObject` Object))
    (bind _input (`/Game/DBDRemake/Common/BPI_Interact.GetInteractionInput` _output_get _role))
    (bind _text (`/Game/DBDRemake/Common/BPI_Interact.GetInteractionText` _output_get _role))
    (`/Game/DBDRemake/UI/UI_Interact.UpdateUIInteraction` (`self.UI_Interact_Ref`) true _input _text)))

(fn `InteractObjectEndOverlap`
  (if (`KismetSystemLibrary.IsValidInterface` (`self.InteractObject`))
    (set `self.InteractObject` null)
    (`/Game/DBDRemake/UI/UI_Interact.UpdateUIInteraction` (`self.UI_Interact_Ref`) false "" "")))