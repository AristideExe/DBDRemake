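; Player interaction component that shows a prompt and triggers interactable objects in range.
; Overlap functions store the current interactable for the locally controlled pawn and update the UI_Interact widget found at BeginPlay with its key and text.
; Either interact input action fires only if it matches the object's declared action, calling Interact locally, then again through a server event flagged as server-side.
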(event `self.ReceiveBeginPlay`
  (bind _foundwidgets (`WidgetBlueprintLibrary.GetAllWidgetsOfClass` "/Game/DBDRemake/UI/UI_Interact.UI_Interact_C" false))
  (set `self.UI_Interact_Ref` (`|GetArrayItem` _foundwidgets)))

(event `EnhancedInput|/Game/DBDRemake/Input/Actions/IA_Interact1`
  (params (ActionValue :type Boolean) (ElapsedSeconds :type "Float (double-precision)") (TriggeredSeconds :type "Float (double-precision)") (InputAction :type "InputAction Object Reference" :default "/Game/DBDRemake/Input/Actions/IA_Interact1.IA_Interact1"))
  (bind _interactobject (`self.InteractObject`))
  (:`Started`
    (if (`KismetSystemLibrary.IsValidInterface` _interactobject)
      (bind _input (`/Game/DBDRemake/Common/BPI_Interact.GetInputAction` _interactobject))
      (if (== _input InputAction)
        (`/Game/DBDRemake/Common/BPI_Interact.Interact` (`self.InteractObject`) (`self.GetOwner`) false :!label _label)
        (`self.SR_Interact` (`self.InteractObject`) (`self.GetOwner`))))))

(event `EnhancedInput|/Game/DBDRemake/Input/Actions/IA_Interact2`
  (params (ActionValue :type Boolean) (ElapsedSeconds :type "Float (double-precision)") (TriggeredSeconds :type "Float (double-precision)") (InputAction :type "InputAction Object Reference" :default "/Game/DBDRemake/Input/Actions/IA_Interact2.IA_Interact2"))
  (bind _interactobject (`self.InteractObject`))
  (:`Started`
    (if (`KismetSystemLibrary.IsValidInterface` _interactobject)
      (bind _input (`/Game/DBDRemake/Common/BPI_Interact.GetInputAction` _interactobject))
      (if (== _input InputAction)
        (goto _label)))))

(event `SR_Interact`
  (params (Target :type "/Game/DBDRemake/Common/BPI_Interact Interface") (Player :type "Actor Object Reference"))
  (`/Game/DBDRemake/Common/BPI_Interact.Interact` Target Player true))

(fn `InteractObjectBeginOverlap`
  (params (Object :type "/Game/DBDRemake/Common/BPI_Interact Interface") (Pawn :type "Pawn Object Reference"))
  (if (== Pawn (`Controller.K2_GetPawn` (`GameplayStatics.GetPlayerController` 0)))
    (bind _output_get (set `self.InteractObject` Object))
    (bind _input (`/Game/DBDRemake/Common/BPI_Interact.GetInteractionInput` _output_get))
    (bind _text (`/Game/DBDRemake/Common/BPI_Interact.GetInteractionText` _output_get))
    (`/Game/DBDRemake/UI/UI_Interact.UpdateUIInteraction` (`self.UI_Interact_Ref`) true _input _text)))

(fn `InteractObjectEndOverlap`
  (if (`KismetSystemLibrary.IsValidInterface` (`self.InteractObject`))
    (set `self.InteractObject` null)
    (`/Game/DBDRemake/UI/UI_Interact.UpdateUIInteraction` (`self.UI_Interact_Ref`) false "" "")))